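; GhostBuilding_BP is a ghost stand-in for a building, holding the active building class, display mesh and construction proxy.
; The spawn event applies the mesh only while the ghost is inactive, and KillGhost clears that state without resetting the mesh component.
; ConstructBuilding spawns the given building at the world origin, then, if the BuildingParent cast succeeds, resets and reactivates the ghost using the spawned actor's mesh and proxy.
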(event `onSpawn`
  (params (displayMesh :type "StaticMesh Object Reference") (buildingClass :type "/Game/Main/Maps/BUILDINGS/BuildingParent Class Reference") (constructionProxy :type "/Game/Main/Blueprints/Construction/ConstructionProxy_BP Class Reference"))
  (if (not (`self.isActive`))
    (set `self.BuildingClass` buildingClass)
    (set `self.ConstructionProxy` constructionProxy)
    (set `self.DisplayMesh` displayMesh)
    (set `self.isActive` true)
    (`StaticMeshComponent.SetStaticMesh` (`self.GhostBuilding_Mesh`) (`self.DisplayMesh`))))

(event `KillGhost`
  (set `self.BuildingClass` null)
  (set `self.ConstructionProxy` null)
  (set `self.DisplayMesh` null)
  (set `self.isActive` false))

(event `Event Construct Building`
  (params (`Main Building` :type "/Game/Main/Maps/BUILDINGS/BuildingParent Class Reference"))
  (bind _returnvalue (`|SpawnActorFromClass` `Main Building` (`KismetMathLibrary.MakeTransform` (0.0 0.0 0.0)) "Undefined" "OverrideRootScale" null null null (`self.ConstructionProxy`) (`self.ControllerRef`) null null null))
  (bind _asbuilding_parent (castclass `/Game/Main/Maps/BUILDINGS/BuildingParent` `Main Building`))
  (`self.KillGhost` self)
  (`self.onSpawn` self (`/Game/Main/Maps/BUILDINGS/BuildingParent.DisplayMeshRef` _returnvalue) _asbuilding_parent (`/Game/Main/Maps/BUILDINGS/BuildingParent.ConstructionProxy` _returnvalue)))

(fn `UserConstructionScript`)