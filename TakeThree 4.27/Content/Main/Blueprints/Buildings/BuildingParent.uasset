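; Parent Blueprint for buildings that lets the player select them in the HUD by clicking.
; On BeginPlay it casts the player controller to PlayerTopDownController, then caches its camera pawn and that pawn's main HUD reference.
; A left mouse click on the actor passes itself to the HUD's UpdateSelection.
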(event `self.ReceiveBeginPlay`
  (bind _asplayer_top_down_controller (cast `/Game/Main/Blueprints/PlayerTopDownController` (`GameplayStatics.GetPlayerController` 0)))
  (bind _thecamerapawn (`/Game/Main/Blueprints/PlayerTopDownController.GetCameraPawn` _asplayer_top_down_controller))
  (bind _output_get (set `self.CameraPawnRef` _thecamerapawn))
  (set `self.HUDRef` (`/Game/Main/Blueprints/CameraPawn.MainHUDRef` _output_get)))

(event `self.ReceiveActorOnClicked`
  (params (ButtonPressed :type "Key Structure"))
  ;[1 1 1] HUD Selection
  (if (== ButtonPressed "LeftMouseButton")
    ;;[1 1 1] Update Selection
    (`/Game/Main/HUDS/MainUI_HUD.UpdateSelection` (`self.HUDRef`) self)))

(fn `UserConstructionScript`)