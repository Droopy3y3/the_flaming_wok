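; Player camera pawn for free navigation, with planar movement, zoom and mouse-driven rotation.
; Move axes offset the actor along its facing, scaled by a fast-move multiplier and a clamped spring-arm-length speed.
; Zoom slides the camera along local X within limits; spring-arm zoom code remains but is unused.
; Gates pass mouse yaw and clamped pitch while Pan X is held, Pan Reset levels pitch, and Tick prints debug text.
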(event `self.ReceiveTick`
  (params (DeltaSeconds :type "Float (single-precision)"))
  (`KismetSystemLibrary.PrintString` "Hello" :!label _label)
  (`KismetSystemLibrary.PrintString` (`KismetStringLibrary.Conv_DoubleToString` (`SpringArmComponent.TargetArmLength` (`self.SpringArm`)))))

(event `self.ReceiveBeginPlay`
  (`|ExecutionSequence`
    (:`then_0`
      (goto _label))))

(event `InputAxis|MoveForward`
  (params (AxisValue :type "Float (single-precision)"))
  ;[1 1 1] Movement X
  (if (not (`self.DisableCameraNav`))
    (bind _returnvalue (`self.MovementX` self (`self.MovementSpeedCalculation`) (`self.FastMoveMultiplier`) AxisValue))
    (`self.K2_SetActorTransform` self _returnvalue false false)))

(event `InputAction|ZoomIn`
  (params (Key :type "Key Structure"))
  (bind _camera (`self.Camera`))
  ;[1 1 1] Zoom
  (:`Pressed`
    (`SceneComponent.K2_SetRelativeLocation` _camera (`KismetMathLibrary.MakeVector` (`KismetMathLibrary.FClamp` (+ (.x (.location (`SceneComponent.GetRelativeTransform` _camera))) (`self.Zoom Sensitivity`)) (`self.OutZoomMax`) (`self.InZoomMax`)) (.y (.location (`SceneComponent.GetRelativeTransform` _camera))) (.z (.location (`SceneComponent.GetRelativeTransform` _camera)))) false false)))

(event `InputAxis|MoveRight`
  (params (AxisValue :type "Float (single-precision)"))
  ;[1 1 1] Movement Y
  (if (not (`self.DisableCameraNav`))
    (bind _returnvalue (`self.MovementY` self AxisValue (`self.MovementSpeedCalculation`) (`self.FastMoveMultiplier`)))
    (`self.K2_SetActorTransform` self _returnvalue false false)))

(event `InputAction|ZoomOut`
  (params (Key :type "Key Structure"))
  (bind _camera (`self.Camera`))
  ;[1 1 1] Zoom
  (:`Pressed`
    (`SceneComponent.K2_SetRelativeLocation` _camera (`KismetMathLibrary.MakeVector` (`KismetMathLibrary.FClamp` (- (.x (.location (`SceneComponent.GetRelativeTransform` _camera))) (`self.Zoom Sensitivity`)) (`self.OutZoomMax`) (`self.InZoomMax`)) (.y (.location (`SceneComponent.GetRelativeTransform` _camera))) (.z (.location (`SceneComponent.GetRelativeTransform` _camera)))) false false)))

(event `InputAxisKey|MouseX`
  (params (AxisValue :type "Float (single-precision)"))
  ;[1 1 1] Pan X
  (`/Engine/EditorBlueprintResources/StandardMacros.Gate` true :!label _label_2
    (:`Exit`
      (`self.K2_SetActorRotation` self (`KismetMathLibrary.MakeRotator` (.roll (`self.K2_GetActorRotation` self)) (.pitch (`self.K2_GetActorRotation` self)) (+ (.yaw (`self.K2_GetActorRotation` self)) (* (`self.Pan Sensitivity`) AxisValue))) false))))

(event `InputAction|Pan X`
  (params (Key :type "Key Structure"))
  ;[1 1 1] Pan X
  (:`Pressed`
    (set `self.DisableCameraNav` false)
    (goto _label_2 :!via `Open`))
  (:`Released`
    (set `self.DisableCameraNav` false)
    (goto _label_2 :!via `Close`)))

(event `InputAxisKey|MouseY`
  (params (AxisValue :type "Float (single-precision)"))
  ;[1 1 1] Pan Y
  (`/Engine/EditorBlueprintResources/StandardMacros.Gate` true :!label _label_3
    (:`Exit`
      (`self.K2_SetActorRotation` self (`KismetMathLibrary.MakeRotator` (.roll (`self.K2_GetActorRotation` self)) (`KismetMathLibrary.FClamp` (+ (.pitch (`self.K2_GetActorRotation` self)) (* (`self.Pan Sensitivity`) AxisValue)) -55.0 15.0) (.yaw (`self.K2_GetActorRotation` self))) false))))

(event `InputAction|Pan X`
  (params (Key :type "Key Structure"))
  ;[1 1 1] Pan Y
  (:`Pressed`
    (set `self.DisableCameraNav` false)
    (goto _label_3 :!via `Open`))
  (:`Released`
    (set `self.DisableCameraNav` false)
    (goto _label_3 :!via `Close`)))

(event `InputAction|Pan Reset`
  (params (Key :type "Key Structure"))
  ;[1 1 1] Pan Reset
  (:`Pressed`
    (`self.K2_SetActorRotation` self (`KismetMathLibrary.MakeRotator` (.roll (`self.K2_GetActorRotation` self)) 0.0 (.yaw (`self.K2_GetActorRotation` self))) false)))

(fn `MovementSpeedCalculation`
  (returns (`Move Sensitivity` :type "Float (double-precision)"))
  (return (`KismetMathLibrary.FClamp` (/ (`SpringArmComponent.TargetArmLength` (`self.SpringArm`)) 100.0) 5.0 20.0)))

(fn `MovementX`
  (params (`Axis Value` :type "Float (double-precision)") (`Move Sensitivity` :type "Float (double-precision)") (`Speed Multiplier` :type "Float (double-precision)"))
  (returns (ReturnValue :type "Transform Structure"))
  (bind _returnvalue (`self.GetTransform` self))
  (return (`KismetMathLibrary.MakeTransform` (+ (`KismetMathLibrary.MakeVector` (.x (`KismetMathLibrary.TransformDirection` _returnvalue (`KismetMathLibrary.MakeVector` (* `Speed Multiplier` (* `Axis Value` `Move Sensitivity`))))) (.y (`KismetMathLibrary.TransformDirection` _returnvalue (`KismetMathLibrary.MakeVector` (* `Speed Multiplier` (* `Axis Value` `Move Sensitivity`)))))) (.location _returnvalue)) (.rotation _returnvalue) (.scale _returnvalue))))

(fn `MovementY`
  (params (`Axis Value` :type "Float (double-precision)") (`Movement Sensitivity` :type "Float (double-precision)") (`Speed Multiplier` :type "Float (double-precision)"))
  (returns (ReturnValue :type "Transform Structure"))
  (bind _returnvalue (`self.GetTransform` self))
  (return (`KismetMathLibrary.MakeTransform` (+ (`KismetMathLibrary.TransformDirection` _returnvalue (`KismetMathLibrary.MakeVector` 0.0 (* `Speed Multiplier` (* `Axis Value` `Movement Sensitivity`)))) (.location _returnvalue)) (.rotation _returnvalue) (.scale _returnvalue))))

(fn `UserConstructionScript`)

(fn `Zoom`
  (params (DirectionIn :type "Float (double-precision)"))
  (locals (ZoomSpeed :type "Float (double-precision)" :default 50.0) (MaxLength :type "Float (double-precision)" :default 2500.0) (`Min Length` :type "Float (double-precision)" :default 20.0))
  (bind _springarm (`self.SpringArm`))
  (set `SpringArmComponent.TargetArmLength` (`KismetMathLibrary.FClamp` (+ (`SpringArmComponent.TargetArmLength` _springarm) (* DirectionIn (`local.ZoomSpeed`))) (`local.Min Length`) (`local.MaxLength`)) _springarm))