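; SelectableObject is an actor that reports itself to the main HUD as the current selection when left-clicked.
; On BeginPlay it casts player controller 0 to PlayerTopDownController, caches its camera pawn and that pawn's main HUD, and prints the pawn for debugging.
; A click retries that lookup if the pawn reference is invalid, then calls the HUD's UpdateSelection and sets IsSelected, which this Blueprint never clears.
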(event `self.ReceiveBeginPlay`
  (`self.SetReferences`))

(event `self.ReceiveActorOnClicked`
  (params (ButtonPressed :type "Key Structure"))
  ;[1 1 1] HUD Selection
  (`/Engine/EditorBlueprintResources/StandardMacros.IsValid` (`self.CameraPawnRef`)
    (:`Is Valid`
      _)
    (:`Is Not Valid`
      (`self.SetReferences`)))
  (if (== ButtonPressed "LeftMouseButton")
    ;;[1 1 1] Update Selection
    (`/Game/Main/HUDS/MainUI_HUD.UpdateSelection` (`self.HUDRef`) self)
    (set `self.IsSelected` true)))

(event `self.ReceiveTick`
  (params (DeltaSeconds :type "Float (single-precision)")))

(fn `SetReferences`
  (bind _asplayer_top_down_controller (cast `/Game/Main/Blueprints/PlayerTopDownController` (`GameplayStatics.GetPlayerController` 0)))
  (bind _thecamerapawn (`/Game/Main/Blueprints/PlayerTopDownController.GetCameraPawn` _asplayer_top_down_controller))
  (bind _output_get (set `self.CameraPawnRef` _thecamerapawn))
  (`KismetSystemLibrary.PrintString` (`KismetStringLibrary.Conv_ObjectToString` _output_get))
  (set `self.HUDRef` (`/Game/Main/Blueprints/CameraPawn.MainHUDRef` _output_get)))

(fn `UserConstructionScript`)